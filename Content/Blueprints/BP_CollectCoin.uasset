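; BP_CollectCoin is a spinning coin pickup that adds to the third-person character's coin count.
; BeginPlay randomly picks the spin direction, and Tick yaws the mesh by a fixed step each frame, independent of delta time.
; When the PickUp component is overlapped, it casts the other actor's instigator to BP_ThirdPersonCharacter, adds AddCoin to its Coin, prints the total and destroys itself.
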(event `self.ReceiveBeginPlay`
  ;[1 1 1] Rotation Coin
  (set `self.Rotation Speed` (`KismetMathLibrary.SelectFloat` 1.5 -1.5 (`KismetMathLibrary.RandomBool`))))

(event `self.ReceiveTick`
  (params (DeltaSeconds :type "Float (single-precision)"))
  ;[1 1 1] Rotation Coin
  (`SceneComponent.K2_AddRelativeRotation` (`self.StaticMesh`) (`KismetMathLibrary.MakeRotator` 0.0 0.0 (`self.Rotation Speed`)) false false))

(event `self.PickUp.OnComponentBeginOverlap`
  (params (OverlappedComponent :type "PrimitiveComponent Object Reference") (OtherActor :type "Actor Object Reference") (OtherComp :type "PrimitiveComponent Object Reference") (OtherBodyIndex :type Integer) (bFromSweep :type Boolean) (SweepResult :type "HitResult Structure (by ref)"))
  ;[1 1 1] Pick Up Coin
  (bind _asbp_third_person_character (cast `/Game/Blueprints/BP_ThirdPersonCharacter` (`self.GetInstigator` OtherActor)))
  (bind _output_get (set `/Game/Blueprints/BP_ThirdPersonCharacter.Coin` (+ (`/Game/Blueprints/BP_ThirdPersonCharacter.Coin` _asbp_third_person_character) (`self.Add Coin`)) _asbp_third_person_character))
  (`KismetSystemLibrary.PrintString` (`KismetStringLibrary.Conv_IntToString` _output_get))
  (`self.K2_DestroyActor`))

(fn `UserConstructionScript`)